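; BP_enemy is a simple enemy actor Blueprint that tracks health and dies when it runs out.
; A takeDamage event subtracts the given amount from Health, then uses the CheckIfDead function to test whether it is at or below zero.
; A dead enemy destroys itself, while a living one prints its remaining health, alongside debug messages on spawn and on each hit.
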(event `self.ReceiveBeginPlay`
  (`KismetSystemLibrary.PrintString` "Hello I am EMENY!"))

(event `takeDamage`
  (params (`By amount` :type "Float (double-precision)"))
  (bind _health (`self.health`))
  ;[1 1 1] take damage and set health
  (`KismetSystemLibrary.PrintString` "OOF")
  (set `self.health` (- (`self.health`) `By amount`))
  ;[1 1 1] Checking if Alive or Dead
  (if (`self.CheckIfDead` _health)
    (`self.K2_DestroyActor`)
    (else
      (`KismetSystemLibrary.PrintString` (`KismetStringLibrary.Conv_DoubleToString` _health) true true (struct :`G` 1.0 :`B` 0.129673 :`A` 1.0)))))

(fn `CheckIfDead`
  (params (Health :type "Float (double-precision)"))
  (returns (IsDead :type Boolean))
  (return (<= Health 0.0)))

(fn `UserConstructionScript`)