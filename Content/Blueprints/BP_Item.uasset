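; BP_Item is an item that can be picked up into a character's hand and dropped, apparently a base or prototype with debug prints.
; Pickup disables the Cube's collision and snaps the item to the handitemsocket_r socket on the given skeletal mesh.
; Drop detaches the Cube, enables physics-only collision and simulation, and applies a small forward-and-up force.
; The primaryAction event is a stub that only prints a message.
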(event `Pickup`
  (params (`Skeletal Mesh` :type "SceneComponent Object Reference"))
  (`KismetSystemLibrary.PrintString` "Calling Pickup" true true (struct :`G` 1.0 :`B` 0.258833 :`A` 1.0))
  (`PrimitiveComponent.SetCollisionEnabled` (`self.Cube`) "NoCollision")
  (`self.K2_AttachToComponent` `Skeletal Mesh` "handitemsocket_r" "SnapToTarget" "SnapToTarget" "KeepRelative"))

(event `self.ReceiveBeginPlay`)

(event `Drop`
  (`KismetSystemLibrary.PrintString` "Calling Drop" true true (struct :`R` 1.0 :`G` 0.012965 :`A` 1.0))
  (`PrimitiveComponent.SetCollisionEnabled` (`self.Cube`) "PhysicsOnly")
  (`PrimitiveComponent.SetSimulatePhysics` (`self.Cube`) true)
  (`SceneComponent.K2_DetachFromComponent` (`self.Cube`) "KeepRelative" "KeepRelative" "KeepRelative" true)
  (`PrimitiveComponent.SetSimulatePhysics` (`self.Cube`) true)
  (`PrimitiveComponent.AddForce` (`self.Cube`) (20.0 0.0 20.0) "None" true))

(event `primaryAction`
  (`KismetSystemLibrary.PrintString` "Calling PrimaryAction"))

(fn `UserConstructionScript`)