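; BP_Enemytester is a test actor that periodically damages every BP_enemy in the level.
; On BeginPlay it gathers all BP_enemy actors, prints their count and calls TakeDamage on each with a small random amount.
; After the loop it prints the array index, waits two seconds and calls its GiveDamage event, repeating the search and damage pass indefinitely.
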(event `giveDamage`
  (bind _outactors (`GameplayStatics.GetAllActorsOfClass` "/Game/Blueprints/BP_enemy.BP_enemy_C" :!label _label)) ; find all enemies
  (`KismetSystemLibrary.PrintString` (`KismetStringLibrary.Concat_StrStr` "" (`KismetStringLibrary.Conv_IntToString` (`KismetArrayLibrary.Array_Length` _outactors)) " enemies in the level"))
  (for (_array_element _array_index) _outactors
    ;[1 1 1] Calls to Take Damage Event in BP_Enemy
    (`/Game/Blueprints/BP_enemy.takeDamage` _array_element (`KismetMathLibrary.RandomFloatInRange` 0.1 0.5)))
  (`KismetSystemLibrary.PrintString` (`KismetStringLibrary.Concat_StrStr` "array index=" (`KismetStringLibrary.Conv_IntToString` _array_index)))
  (`KismetSystemLibrary.Delay` 2.0)
  (`self.giveDamage`))

(event `self.ReceiveBeginPlay`
  (goto _label))

(fn `UserConstructionScript`)